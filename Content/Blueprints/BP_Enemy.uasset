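; BP_Enemy is an enemy actor that moves straight down the Z axis each tick at a rate set by Speedy.
; DestroyEnemy removes it once it falls to a low Z threshold.
; When its Box overlaps a BP_Shoot, it destroys the shot, adds points to the score in GS_Jogo and destroys itself.
; The per-tick movement is not scaled by delta time, so speed depends on frame rate.
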(event OnComponentBeginOverlap(Box)
  (params (OverlappedComponent :type Primitive%20Component%20Object%20Reference) (OtherActor :type Actor%20Object%20Reference) (OtherComp :type Primitive%20Component%20Object%20Reference) (OtherBodyIndex :type Integer) (bFromSweep :type Boolean) (SweepResult :type Hit%20Result%20Structure%20%28by%20ref%29))
  (bind _asbp_shoot (Utilities|Casting|CastToBP_Shoot OtherActor))
  (Actor|DestroyActor _asbp_shoot)
  (bind _asgs_jogo (Utilities|Casting|CastToGS_Jogo (Game|GetGameState)))
  (Default|AddScore _asgs_jogo 1e+01)
  (Actor|DestroyActor))

(event Collision|EventActorBeginOverlap
  (params (OtherActor :type Actor%20Object%20Reference)))

(event EventTick
  (params (DeltaSeconds :type Float%20%28single-precision%29))
  (bind _returnvalue (Transformation|GetActorLocation))
  (Transformation|SetActorLocation (Math|Vector|MakeVector (.x _returnvalue) (.y _returnvalue) (- (.z _returnvalue) (Variables|Default|GetSpeedy))) false false)
  (CallFunction|DestroyEnemy -6e+02))

(fn ConstructionScript)

(fn DestroyEnemy
  (params (ZValue :type Float%20%28single-precision%29))
  (if (<= (.z (Transformation|GetActorLocation)) ZValue)
    (Actor|DestroyActor)))