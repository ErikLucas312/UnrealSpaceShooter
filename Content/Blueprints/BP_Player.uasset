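; BP_Player is the player actor of a shooter: it moves sideways, fires shots and loses lives when enemies hit it.
; Axis input shifts it along Y within fixed bounds, and Fire spawns BP_Shoot at PointShoot.
; Box overlap with a BP_Enemy destroys the enemy and decrements GS_Jogo life, destroying the player when none remain.
; It creates WB_HUD on BeginPlay and copies score and life from GS_Jogo every Tick.
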(event OnComponentBeginOverlap(Box)
  (params (OverlappedComponent :type Primitive%20Component%20Object%20Reference) (OtherActor :type Actor%20Object%20Reference) (OtherComp :type Primitive%20Component%20Object%20Reference) (OtherBodyIndex :type Integer) (bFromSweep :type Boolean) (SweepResult :type Hit%20Result%20Structure%20%28by%20ref%29))
  (bind _asbp_enemy (Utilities|Casting|CastToBP_Enemy OtherActor))
  (Actor|DestroyActor _asbp_enemy)
  (bind _asgs_jogo (Utilities|Casting|CastToGS_Jogo (Game|GetGameState)))
  (bind _liferesult (Default|DecLife _asgs_jogo))
  (if (not (> _liferesult 0))
    (Actor|DestroyActor)))

(event EventBeginPlay
  (bind _returnvalue (UserInterface|CreateWidget "/Game/Interface/WB_HUD.WB_HUD_C"))
  (bind _output_get (Variables|Default|SetHUD _returnvalue))
  (UserInterface|Viewport|AddtoViewport _output_get 0))

(event Collision|EventActorBeginOverlap
  (params (OtherActor :type Actor%20Object%20Reference)))

(event EventTick
  (params (DeltaSeconds :type Float%20%28single-precision%29))
  (bind _hud (Variables|Default|GetHUD))
  (bind _asgs_jogo (Utilities|Casting|CastToGS_Jogo (Game|GetGameState)))
  (Rendering|Components|TextRender|SetText (Variables|/Game/Interface/WB_HUD.WB_HUD_C|GettxtScore _hud) (Utilities|Text|ToText(Float) (Variables|/Game/Blueprints/GS_Jogo.GS_Jogo_C|GetScore _asgs_jogo) "HalfToEven"))
  (Rendering|Components|TextRender|SetText (Variables|/Game/Interface/WB_HUD.WB_HUD_C|GettxtLife _hud) (Utilities|Text|ToText(Integer) (Variables|/Game/Blueprints/GS_Jogo.GS_Jogo_C|GetLife _asgs_jogo))))

(event Input|ActionEvents|InputActionFire
  (params (Key :type Key%20Structure))
  (:Pressed
    (Game|SpawnActorfromClass "/Game/Blueprints/BP_Shoot.BP_Shoot_C" (Math|Transform|MakeTransform (Transformation|GetWorldLocation (Variables|Default|GetPointShoot)) "90.000000, 0, 0") "Undefined" 0 0)))

(event Input|AxisEvents|InputAxisMoveHorizontal
  (params (AxisValue :type Float%20%28single-precision%29))
  (bind _returnvalue (Transformation|GetActorLocation))
  (bind _speed (Variables|Default|GetSpeed))
  (bind _returnvalue_2 (* AxisValue _speed))
  (bind _returnvalue_3 (+ _returnvalue_2 (.y _returnvalue)))
  ;[1 1 1] Movimenta o Player
  (if (and (>= _returnvalue_3 -9e+02) (<= _returnvalue_3 9e+02))
    (Transformation|SetActorLocation (Math|Vector|MakeVector (.x _returnvalue) _returnvalue_3 (.z _returnvalue)) false false)))

(fn ConstructionScript)